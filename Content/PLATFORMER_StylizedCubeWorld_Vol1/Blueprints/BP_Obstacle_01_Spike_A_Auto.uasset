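; Automatic spike trap obstacle that cycles on its own from BeginPlay, with configurable meshes and material set in the construction script.
; Each cycle plays an attenuated sound at the trap and runs a timeline that lerps the spike's relative location between down and up positions, then waits a set duration and repeats.
; Any valid actor that begins overlapping the spike is passed to the attack component's Attack call.
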(event OnComponentBeginOverlap(Spike)
  (params (OverlappedComponent :type Primitive%20Component%20Object%20Reference) (OtherActor :type Actor%20Object%20Reference) (OtherComp :type Primitive%20Component%20Object%20Reference) (OtherBodyIndex :type Integer) (bFromSweep :type Boolean) (SweepResult :type Hit%20Result%20Structure%20%28by%20ref%29))
  (Utilities|IsValid OtherActor
    (:Is%20Valid
      (Class|UAttackComp|Attack (Variables|Default|GetUAttackComp) OtherActor))))

(event Custom|_Spike
  (Audio|SpawnSoundatLocation "/Game/Sounds/Spikes/SC_Spikes.SC_Spikes" (Transformation|GetActorLocation) "0, 0, 0" 1.0 1.0 0.0 "/Game/Sounds/Spikes/SA_Spikes.SA_Spikes" 0)
  (bind _newtrack_0 (Timeline|Spike_ PlayFromStart)
    (:Update
      (Transformation|SetRelativeLocation (Variables|Default|GetSpike) (Math|Vector|Lerp(Vector) (Math|Vector|MakeVector 0.0 0.0 (Variables|Default|GetSpike%20Down)) (Math|Vector|MakeVector 0.0 0.0 (Variables|Default|GetSpike%20Up)) _newtrack_0) false false))
    (:Finished
      (Utilities|FlowControl|Delay (Variables|Default|GetDuration))
      (CallFunction|Spike))))

(event EventBeginPlay
  (CallFunction|Spike))

(event Collision|EventActorBeginOverlap
  (params (OtherActor :type Actor%20Object%20Reference)))

(event EventTick
  (params (DeltaSeconds :type Float%20%28single-precision%29)))

(fn ConstructionScript
  (Rendering|Material|SetMaterial (Variables|Default|GetSpike) 0 (Variables|Default|GetMaterial))
  (Components|StaticMesh|SetStaticMesh (Variables|Default|GetSpike) (Variables|Default|GetStatic%20Mesh%20Spike))
  (Components|StaticMesh|SetStaticMesh (Variables|Default|GetBase) (Variables|Default|GetStatic%20Mesh%20Base)))